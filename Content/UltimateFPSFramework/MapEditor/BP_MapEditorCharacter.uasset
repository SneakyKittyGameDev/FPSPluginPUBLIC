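; Player character for the in-game map editor, flying through the level and editing placed actors.
; Movement, look and mouse-wheel speed go to SKGMapEditorCharacterMovement; holding right mouse enters movement mode.
; Outside that mode, click and hotkeys drive SKGMapEditorHandler to grab, switch gizmos, duplicate or delete.
; On begin play or possession it initializes the handler and shows W_MapEditor locally; Y returns to the previous pawn.
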(event `self.ReceiveBeginPlay`
  (`KismetSystemLibrary.Delay` 0.2 :!label _label)
  (`self.HandleHUD`))

(event `self.ReceivePossessed`
  (params (NewController :type "Controller Object Reference"))
  (goto _label))

(event `InputAxis|MoveForward`
  (params (AxisValue :type "Float (single-precision)"))
  (bind _asskgmap_editor_character_movement (cast `SKGMapEditorCharacterMovement` (`self.CharacterMovement`)))
  (`SKGMapEditorCharacterMovement.MoveForward` _asskgmap_editor_character_movement AxisValue))

(event `InputAxis|MoveRight`
  (params (AxisValue :type "Float (single-precision)"))
  (bind _asskgmap_editor_character_movement (cast `SKGMapEditorCharacterMovement` (`self.CharacterMovement`)))
  (`SKGMapEditorCharacterMovement.MoveRight` _asskgmap_editor_character_movement AxisValue))

(event `InputAxis|MoveUp`
  (params (AxisValue :type "Float (single-precision)"))
  (bind _asskgmap_editor_character_movement (cast `SKGMapEditorCharacterMovement` (`self.CharacterMovement`)))
  (`SKGMapEditorCharacterMovement.MoveUp` _asskgmap_editor_character_movement AxisValue))

(event `Key|Y`
  (params (Key :type "Key Structure"))
  (:`Pressed`
    (bind _asskgmap_editor_character_movement (cast `SKGMapEditorCharacterMovement` (`self.CharacterMovement`)))
    (`SKGMapEditorCharacterMovement.EnterMovementMode` _asskgmap_editor_character_movement true)
    (`Widget.RemoveFromParent` (`self.W_MapEditor`))
    (`SKGMapEditorHandlerComponent.UnpossessToReturnPawn` (`self.SKGMapEditorHandler`))))

(event `InputAxis|Turn`
  (params (AxisValue :type "Float (single-precision)"))
  (bind _asskgmap_editor_character_movement (cast `SKGMapEditorCharacterMovement` (`self.CharacterMovement`)))
  (`SKGMapEditorCharacterMovement.Turn` _asskgmap_editor_character_movement AxisValue))

(event `InputAxis|LookUp`
  (params (AxisValue :type "Float (single-precision)"))
  (bind _asskgmap_editor_character_movement (cast `SKGMapEditorCharacterMovement` (`self.CharacterMovement`)))
  (`SKGMapEditorCharacterMovement.LookUp` _asskgmap_editor_character_movement AxisValue))

(event `Key|RightMouseButton`
  (params (Key :type "Key Structure"))
  (bind _charactermovement (`self.CharacterMovement`))
  (:`Pressed`
    (bind _asskgmap_editor_character_movement (cast `SKGMapEditorCharacterMovement` _charactermovement))
    (`SKGMapEditorCharacterMovement.EnterMovementMode` _asskgmap_editor_character_movement true))
  (:`Released`
    (bind _asskgmap_editor_character_movement_2 (cast `SKGMapEditorCharacterMovement` _charactermovement))
    (`SKGMapEditorCharacterMovement.EnterMovementMode` _asskgmap_editor_character_movement_2 false)))

(event `Key|LeftMouseButton`
  (params (Key :type "Key Structure"))
  (bind _w_mapeditor (`self.W_MapEditor`))
  (:`Pressed`
    (bind _asskgmap_editor_character_movement (cast `SKGMapEditorCharacterMovement` (`self.CharacterMovement`)))
    (if (not (`SKGMapEditorCharacterMovement.InMovementMode` _asskgmap_editor_character_movement))
      (`SKGMapEditorHandlerComponent.Grab` (`self.SKGMapEditorHandler`))))
  (:`Released`
    (`SKGMapEditorHandlerComponent.Release` (`self.SKGMapEditorHandler`))
    (`/Engine/EditorBlueprintResources/StandardMacros.IsValid` _w_mapeditor
      (:`Is Valid`
        (`/Game/UltimateFPSFramework/MapEditor/UI/W_MapEditor.UpdateUI` _w_mapeditor)))))

(event `Key|E`
  (params (Key :type "Key Structure"))
  (:`Pressed`
    (bind _asskgmap_editor_character_movement (cast `SKGMapEditorCharacterMovement` (`self.CharacterMovement`)))
    (if (not (`SKGMapEditorCharacterMovement.InMovementMode` _asskgmap_editor_character_movement))
      (`SKGMapEditorHandlerComponent.ShowRotation` (`self.SKGMapEditorHandler`))
      (`/Game/UltimateFPSFramework/MapEditor/UI/W_MapEditor.SwitchGizmoType` (`self.W_MapEditor`)))))

(event `Key|R`
  (params (Key :type "Key Structure"))
  (:`Pressed`
    (bind _asskgmap_editor_character_movement (cast `SKGMapEditorCharacterMovement` (`self.CharacterMovement`)))
    (if (not (`SKGMapEditorCharacterMovement.InMovementMode` _asskgmap_editor_character_movement))
      (`SKGMapEditorHandlerComponent.ShowScale` (`self.SKGMapEditorHandler`))
      (`/Game/UltimateFPSFramework/MapEditor/UI/W_MapEditor.SwitchGizmoType` (`self.W_MapEditor`)))))

(event `Key|W`
  (params (Key :type "Key Structure"))
  (:`Pressed`
    (bind _asskgmap_editor_character_movement (cast `SKGMapEditorCharacterMovement` (`self.CharacterMovement`)))
    (if (not (`SKGMapEditorCharacterMovement.InMovementMode` _asskgmap_editor_character_movement))
      (`SKGMapEditorHandlerComponent.ShowMovement` (`self.SKGMapEditorHandler`))
      (`/Game/UltimateFPSFramework/MapEditor/UI/W_MapEditor.SwitchGizmoType` (`self.W_MapEditor`)))))

(event `Key|Delete`
  (params (Key :type "Key Structure"))
  (:`Pressed`
    (bind _asskgmap_editor_character_movement (cast `SKGMapEditorCharacterMovement` (`self.CharacterMovement`)))
    (if (not (`SKGMapEditorCharacterMovement.InMovementMode` _asskgmap_editor_character_movement))
      (`SKGMapEditorHandlerComponent.DeleteActor` (`self.SKGMapEditorHandler`)))))

(event `Key|G`
  (params (Key :type "Key Structure"))
  (:`Pressed`
    (bind _asskgmap_editor_character_movement (cast `SKGMapEditorCharacterMovement` (`self.CharacterMovement`)))
    (if (not (`SKGMapEditorCharacterMovement.InMovementMode` _asskgmap_editor_character_movement))
      (`SKGMapEditorHandlerComponent.DuplicateActor` (`self.SKGMapEditorHandler`) false))))

(event `Key|MouseScrollUp`
  (params (Key :type "Key Structure"))
  (:`Pressed`
    (bind _asskgmap_editor_character_movement (cast `SKGMapEditorCharacterMovement` (`self.CharacterMovement`)))
    (`SKGMapEditorCharacterMovement.IncreaseSpeedMultiplier` _asskgmap_editor_character_movement 0.2)))

(event `Key|MouseScrollDown`
  (params (Key :type "Key Structure"))
  (:`Pressed`
    (bind _asskgmap_editor_character_movement (cast `SKGMapEditorCharacterMovement` (`self.CharacterMovement`)))
    (`SKGMapEditorCharacterMovement.DecreaseSpeedMultiplier` _asskgmap_editor_character_movement 0.2)))

(fn `HandleHUD`
  (bind _w_mapeditor (`self.W_MapEditor`))
  (`SKGMapEditorHandlerComponent.Init` (`self.SKGMapEditorHandler`))
  (if (`self.IsLocallyControlled`)
    (`/Engine/EditorBlueprintResources/StandardMacros.IsValid` _w_mapeditor
      (:`Is Valid`
        (if (not (`Widget.IsInViewport` _w_mapeditor))
          (`UserWidget.AddToViewport` (`self.W_MapEditor`) 0)))
      (:`Is Not Valid`
        (bind _returnvalue (`|CreateWidget` "/Game/UltimateFPSFramework/MapEditor/UI/W_MapEditor.W_MapEditor_C" null (`self.SKGMapEditorHandler`)))
        (bind _output_get (set `self.W_MapEditor` _returnvalue))
        (`UserWidget.AddToViewport` _output_get 0)))))

(fn `UserConstructionScript`)