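; BP_556 is a projectile Blueprint, apparently for 5.56 rounds, that handles impacts with ricochet and penetration.
; On impact, an angle above a fixed threshold triggers a ricochet with slight speed loss; otherwise it penetrates, losing velocity in proportion to object thickness.
; It then sends OnHitMessage to the hit actor and spawns delayed impact effects and sound from the surface's SKGPhysicalMaterial.
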(event `self.OnProjectileImpact`
  (params (HitResult :type "HitResult Structure (by ref)") (HitObjectThickness :type "Float (single-precision)") (Angle :type "Float (single-precision)") (PenetrationLocation :type "Vector Structure (by ref)"))
  (bind (_bblockinghit _binitialoverlap _time _distance _location _impactpoint _normal _impactnormal _physmat _hitactor) (`GameplayStatics.BreakHitResult` HitResult))
  (if (> Angle 15.0)
    (`self.PerformRicochet` HitResult 0.9)
    (else
      (`self.SetAtPenetratedLocation` PenetrationLocation (`KismetMathLibrary.FClamp` (- 1.0 (`KismetMathLibrary.NormalizeToRange` HitObjectThickness 0.0 20.0))))))
  (message `SKGHitInterface.OnHit` _hitactor HitResult self)
  (bind _asskgphysical_material (cast `SKGPhysicalMaterial` _physmat))
  (`SKGFPSStatics.SpawnImpactEffectSoundDelayed` HitResult (`SKGPhysicalMaterial.ProjectileImpactEffects` _asskgphysical_material)))

(fn `UserConstructionScript`)