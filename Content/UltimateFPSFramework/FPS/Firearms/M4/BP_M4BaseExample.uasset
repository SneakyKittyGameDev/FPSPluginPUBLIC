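; Example M4 firearm for the FPS framework, serving as reference firing and reloading logic built on helper functions.
; Fire spawns a projectile, updates ammo and muzzle heat, applies procedural recoil and plays effects, with a timer repeating shots for burst and full auto.
; Shots and reloads run locally first, then replicate via server and multicast events that skip the local player.
; Reload montages follow bolt state, and equip events toggle any stabilizer.
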(event `Equip_1`
  (bind _returnvalue (`self.GetStabilizerComponent`))
  ;[0 1 0] Run Logic for when Equipped
  (`/Engine/EditorBlueprintResources/StandardMacros.IsValid` _returnvalue
    (:`Is Valid`
      (`KismetSystemLibrary.Delay` 0.5)
      (`SKGFirearmStabilizerComponent.Enable` _returnvalue))))

(event `UnEquip_1`
  (bind _returnvalue (`self.GetStabilizerComponent`))
  ;[0 1 0] Run Logic for when UnEquipped
  (`|PlayMontage` (`SKGCharacterComponent.GetInUseMesh` (`self.GetCharacterComponent`)) "/Game/UltimateFPSFramework/FPS/Assets/Firearm/M4/Animation/Character/AM_M4_Arms_Equip.AM_M4_Arms_Equip" 1.0 0.0 "UnEquip"
    (:`then`
      (`/Engine/EditorBlueprintResources/StandardMacros.IsValid` _returnvalue
        (:`Is Valid`
          (`SKGFirearmStabilizerComponent.Disable` _returnvalue))))))

(event `self.ReceiveBeginPlay`
  ;[0 1 0] Example Firing/Reloading logic to be used as a reference using helper functions
)

(event `self.Fire`
  (bind _lastfiredtransform (`self.LastFiredTransform`))
  ;[0 1 0] Example Firing/Reloading logic to be used as a reference using helper functions
  (if (`self.CanFire`)
    (`self.HandleMuzzleHeat`)
    (bind _returnvalue (`self.GetFirearmStats`))
    (bind _output_get (set `self.LastFiredTransform` (`self.GetMuzzleProjectileSocketTransform` 100.0 (* (`.AccuracyMultiplier` (break `SKGFirearmStats` _returnvalue)) (`self.AccuracyMOA`)))))
    (`self.HandleProjectileFireAndRecoil` _output_get)
    (`self.PlayFireEffect`)
    (`self.PlayFireSound`)
    (bind _sectionname (`self.GetFireMontageSection`))
    (`|PlayMontage` (`self.FirearmMesh`) "/Game/UltimateFPSFramework/FPS/Assets/Firearm/M4/Animation/Firearm/AM_M4_Fire.AM_M4_Fire" 1.0 0.0 _sectionname
      (:`then`
        (`/Engine/EditorBlueprintResources/ActorMacros.Switch Has Authority`
          (:`Authority`
            (`self.Multi_Fire` _lastfiredtransform))
          (:`Remote`
            (`self.Server_Fire` _lastfiredtransform)))
        (switch `ESKGFirearmFireMode` (`self.FireMode`)
          (:`Burst`
            (bind _result (`/Engine/EditorBlueprintResources/StandardMacros.IncrementInt` (`self.BurstCounter`))
              (:`  `
                (if (>= _result (`self.BurstCount`))
                  (`self.StopFire`)
                  (set `self.BurstCounter` 0)
                  (else
                    (bind _returnvalue_2 (`KismetSystemLibrary.K2_SetTimerDelegate` (delegate `self.Fire`) (`self.GetCycleRate` false) true :!label _label))
                    (set `self.T_FAHandle` _returnvalue_2))))))
          (:`FullAuto`
            (goto _label)))))
    (else
      (`self.StopFire`))))

(event `Server_Fire`
  (params (MuzzleTransform :type "SKGProjectileTransform Structure"))
  ;[0 1 0] Example Firing/Reloading logic to be used as a reference using helper functions
  (`self.Multi_Fire` MuzzleTransform))

(event `Multi_Fire`
  (params (MuzzleTransform :type "SKGProjectileTransform Structure"))
  ;[0 1 0] Example Firing/Reloading logic to be used as a reference using helper functions
  (`SKGCharacterComponent.IsLocallyControlled` (`self.GetCharacterComponent`)
    (:`False`
      (`self.HandleMuzzleHeat`)
      (`self.HandleProjectileFireAndRecoil` MuzzleTransform)
      (`self.PlayFireEffect`)
      (`self.PlayFireSound`)
      (bind _sectionname (`self.GetFireMontageSection`))
      (`|PlayMontage` (`self.FirearmMesh`) "/Game/UltimateFPSFramework/FPS/Assets/Firearm/M4/Animation/Firearm/AM_M4_Fire.AM_M4_Fire" 1.0 0.0 _sectionname))))

(event `self.StopFire`
  ;[0 1 0] Example Firing/Reloading logic to be used as a reference using helper functions
  (`KismetSystemLibrary.K2_ClearAndInvalidateTimerHandle` (`self.T_FAHandle`)))

(event `self.Reload`
  ;[0 1 0] Example Firing/Reloading logic to be used as a reference using helper functions
  (`self.StopFire`)
  (`self.StartReload`)
  (`SKGCharacterAnimInstance.SetIsReloading` (`SKGCharacterComponent.GetAnimationInstance` (`self.GetCharacterComponent`)) true 0.35)
  (set `self.Reloading` true)
  (`/Engine/EditorBlueprintResources/ActorMacros.Switch Has Authority`
    (:`Authority`
      (`self.Multi_Reload`))
    (:`Remote`
      (`self.Server_Reload`))))

(event `StartReload`
  (bind _returnvalue (`self.GetCharacterComponent`))
  ;[0 1 0] Example Firing/Reloading logic to be used as a reference using helper functions
  (bind (_firearm _character _section) (`self.GetReloadMontages`))
  (`|PlayMontage` (`self.FirearmMesh`) _firearm 1.0 0.0 _section
    (:`then`
      (`|PlayMontage` (`SKGCharacterComponent.GetInUseMesh` _returnvalue) _character 1.0 0.0 _section
        (:`then`
          (`SKGCharacterAnimInstance.SetIsReloading` (`SKGCharacterComponent.GetAnimationInstance` _returnvalue) true 0.35))))))

(event `Server_Reload`
  ;[0 1 0] Example Firing/Reloading logic to be used as a reference using helper functions
  (`self.Multi_Reload`))

(event `Multi_Reload`
  ;[0 1 0] Example Firing/Reloading logic to be used as a reference using helper functions
  (`SKGCharacterComponent.IsLocallyControlled` (`self.GetCharacterComponent`)
    (:`False`
      (`self.StartReload`))))

(event `ReloadCompleted`
  (bind _returnvalue (`self.GetCharacterComponent`))
  (bind _returnvalue_2 (- (`self.TotalAmmo`) (- (`self.MagazineCapacity`) (`self.MagazineAmmo`))))
  ;[0 1 0] Example Firing/Reloading logic to be used as a reference using helper functions
  (set `self.Reloading` false)
  (set `self.BoltOpen` false)
  (`SKGCharacterComponent.IsLocallyControlled` _returnvalue
    (:`True`
      (`SKGCharacterAnimInstance.SetIsReloading` (`SKGCharacterComponent.GetAnimationInstance` _returnvalue) false 0.35))
    (:`False`
      _))
  (`/Engine/EditorBlueprintResources/ActorMacros.Switch Has Authority`
    (:`Authority`
      _)
    (:`Remote`
      _))
  (if (< _returnvalue_2 0)
    (set `self.TotalAmmo` 0)
    (else
      (set `self.TotalAmmo` _returnvalue_2)))
  (if (> (`self.MagazineCapacity`) (`self.TotalAmmo`))
    (set `self.MagazineAmmo` (`self.TotalAmmo`))
    (else
      (set `self.MagazineAmmo` (`self.MagazineCapacity`))))
  (`SKGCharacterAnimInstance.SetIsReloading` (`SKGCharacterComponent.GetAnimationInstance` (`self.GetCharacterComponent`)) false 0.35))

(fn `CanFire`
  (returns (CanFire :type Boolean))
  (return (and (`|EnumInequality` (`self.FireMode`) "Safe") (> (`self.MagazineAmmo`) 0) (not (`self.Reloading`)))))

(fn `GetFireMontageSection`
  (returns (SectionName :type Name))
  (if (< (`self.MagazineAmmo`) 1)
    (return "FireEmpty")
    (else
      (return "Fire"))))

(fn `GetReloadMontages`
  (returns (Firearm :type "AnimMontage Object Reference") (Character :type "AnimMontage Object Reference") (Section :type Name))
  (if (`self.BoltOpen`)
    (return "/Game/UltimateFPSFramework/FPS/Assets/Firearm/M4/Animation/Firearm/AM_M4_Reload.AM_M4_Reload" "/Game/UltimateFPSFramework/FPS/Assets/Firearm/M4/Animation/Character/AM_M4_Arms_Reload.AM_M4_Arms_Reload" "Dry")
    (else
      (return "/Game/UltimateFPSFramework/FPS/Assets/Firearm/M4/Animation/Firearm/AM_M4_Reload.AM_M4_Reload" "/Game/UltimateFPSFramework/FPS/Assets/Firearm/M4/Animation/Character/AM_M4_Arms_Reload.AM_M4_Arms_Reload" "Tactical"))))

(fn `HandleFireAmmo`
  (`/Engine/EditorBlueprintResources/StandardMacros.DecrementInt` (`self.MagazineAmmo`)
    (:`  `
      (if (< (`self.MagazineAmmo`) 1)
        (set `self.BoltOpen` true)
        (else
          (set `self.BoltOpen` false))))))

(fn `HandleMuzzleHeat`
  (bind _returnvalue (`self.GetMuzzleDevice`))
  (bind _returnvalue_barrel (break `SKGFirearmCachedParts` (`self.GetCachedComponents`)))
  (`/Engine/EditorBlueprintResources/StandardMacros.IsValid` _returnvalue
    (:`Is Valid`
      (`SKGMuzzle.FiredShot` _returnvalue)
      (`/Engine/EditorBlueprintResources/StandardMacros.IsValid` _returnvalue_barrel
        (:`Is Valid`
          (bind _asskgbarrel (cast `SKGBarrel` (`SKGAttachmentComponent.GetAttachment` _returnvalue_barrel)))
          (`SKGBarrel.FiredShot` _asskgbarrel))))))

(fn `HandleProjectileFireAndRecoil`
  (params (MuzzleTransform :type "SKGProjectileTransform Structure"))
  (locals (RecoilADSMultiplier :type "Float (double-precision)" :default 1.2) (RecoilHIPMultiplier :type "Float (double-precision)" :default 2.0))
  (bind _returnvalue (`|SpawnActorFromClass` (`self.ProjectileClass`) (`SKGFPSStatics.ProjectileTransformToTransform` MuzzleTransform) "AlwaysSpawn" "OverrideRootScale" self null))
  (bind _returnvalue_2 (`self.GetFirearmStats`))
  (`SKGProjectile.ActivateProjectile` _returnvalue (`.MuzzleVelocityMultiplier` (break `SKGFirearmStats` _returnvalue_2)))
  (`self.HandleFireAmmo`)
  (`/Engine/EditorBlueprintResources/StandardMacros.IsValid` (`self.GetCharacterComponent`)
    (:`Is Valid`
      (if (`self.IsStabilized`)
        (set `local.RecoilADSMultiplier` (* (`local.RecoilADSMultiplier`) 0.5))
        (set `local.RecoilHIPMultiplier` (* (`local.RecoilHIPMultiplier`) 0.5)))
      (`SKGCharacterComponent.IsAiming` (`self.GetCharacterComponent`)
        (:`True`
          (`self.PerformProceduralRecoil` (`local.RecoilADSMultiplier`) false true))
        (:`False`
          (`self.PerformProceduralRecoil` (`local.RecoilHIPMultiplier`) false))))))

(fn `PlayFireEffect`
  (bind _returnvalue (`self.GetFireNiagaraSystem`))
  (`/Engine/EditorBlueprintResources/StandardMacros.IsValid` _returnvalue
    (:`Is Valid`
      (bind _returnvalue_2 (`SKGFirearmPartsInterface.GetMuzzleSocketTransform`))
      (`NiagaraFunctionLibrary.SpawnSystemAtLocation` _returnvalue (.location _returnvalue_2) (.rotation _returnvalue_2)))))

(fn `PlayFireSound`
  (bind _returnvalue (`SKGFirearmPartsInterface.GetMuzzleSocketTransform`))
  (`self.IsSuppressed`
    (:`True`
      (`SKGFPSStatics.PlaySoundDelayed` self (.location _returnvalue) (make `SKGSoundSettings` "/Game/UltimateFPSFramework/FPS/Assets/Firearm/Audio/Shooting/SC_FireSuppressed.SC_FireSuppressed")))
    (:`False`
      (`SKGFPSStatics.PlaySoundDelayed` self (.location _returnvalue) (make `SKGSoundSettings` "/Game/UltimateFPSFramework/FPS/Assets/Firearm/Audio/Shooting/SC_Fire.SC_Fire")))))

(fn `UserConstructionScript`)