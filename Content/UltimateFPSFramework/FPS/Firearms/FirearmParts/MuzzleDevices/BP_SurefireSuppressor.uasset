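; Suppressor muzzle device Blueprint for the FPS framework's Surefire suppressor, adding a heat smoke effect driven by barrel heat.
; The Niagara smoke starts inactive, and muzzle temperature changes are normalized to a 0–1 value that activates it and feeds its MuzzleTemp parameter.
; Smoke shuts off when that value reaches zero or an attachment occupies the AttachmentCover, and updates only run while that cover reference is valid.
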(event `self.ReceiveBeginPlay`
  (`ActorComponent.Deactivate` (`self.NS_HeatSmoke`)))

(event `self.MuzzleTemperatureChanged`
  (params (NewMuzzleTemperature :type "Float (single-precision)"))
  (bind _ns_heatsmoke (`self.NS_HeatSmoke`))
  (bind _attachment_cover (`self.Attachment_Cover`))
  (bind _returnvalue (`KismetMathLibrary.FClamp` (`KismetMathLibrary.NormalizeToRange` NewMuzzleTemperature 50.0 700.0)))
  (`/Engine/EditorBlueprintResources/StandardMacros.IsValid` _attachment_cover
    (:`Is Valid`
      (if (`SKGAttachmentComponent.HasAttachment` _attachment_cover)
        (if (`ActorComponent.IsActive` _ns_heatsmoke)
          (`ActorComponent.Deactivate` _ns_heatsmoke))
        (elif (> _returnvalue 0.0)
          (if (not (`ActorComponent.IsActive` (`self.NS_HeatSmoke`)))
            (`ActorComponent.Activate` (`self.NS_HeatSmoke`) false))
          (`NiagaraComponent.SetVariableFloat` (`self.NS_HeatSmoke`) "MuzzleTemp" _returnvalue)
          (elif (`ActorComponent.IsActive` (`self.NS_HeatSmoke`))
            (`ActorComponent.Deactivate` (`self.NS_HeatSmoke`))))))))

(fn `UserConstructionScript`)