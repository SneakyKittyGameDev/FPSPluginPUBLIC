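; BP_LightLaser is a light/laser firearm part that drives the visuals of its flashlight and supplies grip socket, animation index, sway and shake settings.
; BeginPlay creates dynamic materials for the lens, beam and blinder, starting beam and blinder transparent.
; Toggle events switch lens glow and beam/blinder visibility, while power changes scale their opacity.
; Infrared mode changes adjust lens intensity according to infrared and night vision state.
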(event `self.ReceiveBeginPlay`
  (bind _returnvalue (`PrimitiveComponent.CreateDynamicMaterialInstance` (`self.StaticMesh`) 1 null "None"))
  (set `self.LightLensMaterial` _returnvalue)
  (bind _returnvalue_2 (`PrimitiveComponent.CreateDynamicMaterialInstance` (`self.LightBeam`) 0 null "None"))
  (`PrimitiveComponent.SetMaterial` (`self.LightBeam`) 0 _returnvalue_2)
  (`MaterialInstanceDynamic.SetScalarParameterValue` _returnvalue_2 "Opacity" (* 0.0 (`self.LightBeamOpacityMultiplier`)))
  (bind _returnvalue_3 (`PrimitiveComponent.CreateDynamicMaterialInstance` (`self.LightBlinder`) 0 null "None"))
  (`PrimitiveComponent.SetMaterial` (`self.LightBlinder`) 0 _returnvalue_3)
  (`MaterialInstanceDynamic.SetScalarParameterValue` _returnvalue_3 "Opacity" 0.0))

(event `self.OnLightToggled`
  (params (bOn :type Boolean))
  (bind _lightblinder (`self.LightBlinder`))
  (bind _lightlensmaterial (`self.LightLensMaterial`))
  (bind _lightlensmaterial_2 (`self.LightLensMaterial`))
  (if bOn
    (`SceneComponent.SetHiddenInGame` _lightblinder false false)
    (`SceneComponent.SetHiddenInGame` (`self.LightBeam`) false false)
    (`/Engine/EditorBlueprintResources/StandardMacros.IsValid` _lightlensmaterial_2
      (:`Is Valid`
        (`MaterialInstanceDynamic.SetScalarParameterValue` _lightlensmaterial_2 "LightOn" 1.0)))
    (else
      (`SceneComponent.SetHiddenInGame` _lightblinder true false)
      (`SceneComponent.SetHiddenInGame` (`self.LightBeam`) true false)
      (`/Engine/EditorBlueprintResources/StandardMacros.IsValid` _lightlensmaterial
        (:`Is Valid`
          (`MaterialInstanceDynamic.SetScalarParameterValue` _lightlensmaterial "LightOn" 0.0))))))

(event `self.OnLightPowerChanged`
  (params (NewPower :type "Float (single-precision)"))
  (bind _asmaterial_instance_dynamic (cast `MaterialInstanceDynamic` (`PrimitiveComponent.GetMaterial` (`self.LightBeam`) 0))
    (:`then`
      (`MaterialInstanceDynamic.SetScalarParameterValue` _asmaterial_instance_dynamic "Opacity" (* NewPower (`self.LightBeamOpacityMultiplier`))))
    (:`CastFailed`
      _))
  (bind _asmaterial_instance_dynamic_2 (cast `MaterialInstanceDynamic` (`PrimitiveComponent.GetMaterial` (`self.LightBlinder`) 0)))
  (`MaterialInstanceDynamic.SetScalarParameterValue` _asmaterial_instance_dynamic_2 "Opacity" (* NewPower (`self.LightBlinderOpacityMultiplier`))))

(event `self.OnInfraredModeChanged`
  (params (bInInfrared :type Boolean) (bIsNightVisionOn :type Boolean))
  (bind _lightlensmaterial (`self.LightLensMaterial`))
  (if (and bInInfrared bIsNightVisionOn)
    (`MaterialInstanceDynamic.SetScalarParameterValue` _lightlensmaterial "Intensity" 100.0)
    (elif bIsNightVisionOn
      (`MaterialInstanceDynamic.SetScalarParameterValue` _lightlensmaterial "Intensity" 5000.0)
      (else
        (`MaterialInstanceDynamic.SetScalarParameterValue` _lightlensmaterial "Intensity" 50.0)))))

(fn `GetAnimationIndex`
  (returns (ReturnValue :type Integer))
  (return 3))

(fn `GetCurveAndShakeSettings`
  (returns (ReturnValue :type "SKGCurveAndShakeSettings Structure"))
  (return (`self.SKGCurve and Shake Settings`)))

(fn `GetGripSocketName`
  (returns (ReturnValue :type Name))
  (return "S_Handheld_LightLaser"))

(fn `GetSwayMultiplier`
  (returns (ReturnValue :type "Float (single-precision)"))
  (return 1.0))

(fn `UserConstructionScript`)