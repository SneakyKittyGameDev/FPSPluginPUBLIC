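; BP_SteelTarget is a steel popper target that falls when hit and pops back up after a delay.
; On hit, it plays the down animation on its skeletal mesh, sets TargetDown and starts a one-shot reset timer.
; The timer clears the flag and plays the up animation, and the flag makes the target ignore hits until that reset.
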(event `self.OnHit`
  (params (HitResult :type "HitResult Structure (by ref)") (Projectile :type "Actor Object Reference"))
  (if (not (`self.TargetDown`))
    (`SkeletalMeshComponent.PlayAnimation` (`self.SkeletalMesh`) "/Game/UltimateFPSFramework/FPS/Assets/Maps/ShootHouse/Assets/Targets/SteelPopper/A_SteelPopper_Down.A_SteelPopper_Down" false)
    (set `self.TargetDown` true)
    (`KismetSystemLibrary.K2_SetTimerDelegate` (delegate `Reset`) (`self.ResetDelay`))))

(event `Reset`
  (set `self.TargetDown` false)
  (`SkeletalMeshComponent.PlayAnimation` (`self.SkeletalMesh`) "/Game/UltimateFPSFramework/FPS/Assets/Maps/ShootHouse/Assets/Targets/SteelPopper/A_SteelPopper_Up.A_SteelPopper_Up" false))

(fn `UserConstructionScript`)