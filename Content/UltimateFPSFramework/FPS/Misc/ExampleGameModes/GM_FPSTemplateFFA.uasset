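; Free-for-all example game mode for the FPS template that spawns a character for each player who joins.
; BeginPlay caches all FPSTemplateSpawnPoint actors, and PostLogin passes each new player controller to SpawnPlayer.
; SpawnPlayer picks a random spawn point, spawns an ExampleFPSTemplateCharacter there with collision adjustment and has the controller possess it.
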(event `self.ReceiveBeginPlay`
  (bind _outactors (`GameplayStatics.GetAllActorsOfClass` "/Game/UltimateFPSFramework/FPS/Misc/ExampleGameModes/FPSTemplateSpawnPoint.FPSTemplateSpawnPoint_C"))
  (set `self.SpawnPoints` _outactors))

(event `self.K2_PostLogin`
  (params (NewPlayer :type "PlayerController Object Reference"))
  (`self.SpawnPlayer` NewPlayer))

(event `SpawnPlayer`
  (params (NewPlayer :type "PlayerController Object Reference"))
  (bind _outitem (`KismetArrayLibrary.Array_Random` (`self.SpawnPoints`)))
  (`/Engine/EditorBlueprintResources/StandardMacros.IsValid` NewPlayer
    (:`Is Valid`
      (`/Engine/EditorBlueprintResources/StandardMacros.IsValid` _outitem
        (:`Is Valid`
          (bind _returnvalue (`|SpawnActorFromClass` "/Game/UltimateFPSFramework/FPS/CharacterRelated/ExampleFPSTemplateCharacter.ExampleFPSTemplateCharacter_C" (`self.GetTransform` _outitem) "AdjustIfPossibleButAlwaysSpawn" "OverrideRootScale" null null))
          (`Controller.Possess` NewPlayer _returnvalue))))))

(fn `UserConstructionScript`)